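; Player character Blueprint for a 2D side-scrolling flipbook game, handling movement, jumping, attacking and pausing through Enhanced Input.
; BeginPlay adds the mapping context; movement runs along world X and flips control yaw to face the travel direction.
; Attack jumps the animation instance to its Attack node, gated until a flipbook-length delay ends, while Pause opens a menu widget.
; Hitcheak scans hitbox overlaps, but its damage call is disconnected and nothing here calls it.
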(event `self.ReceiveBeginPlay`
  (`self.NewFunction_0`))

(event `EnhancedInput|/Game/Input/Controls/Move_IA`
  (params (ActionValue :type "Float (double-precision)") (ElapsedSeconds :type "Float (double-precision)") (TriggeredSeconds :type "Float (double-precision)") (InputAction :type "InputAction Object Reference" :default "/Game/Input/Controls/Move_IA.Move_IA"))
  (:`Triggered`
    (`self.NewFunction` ActionValue ActionValue)))

(event `EnhancedInput|/Game/Input/Controls/Jump_IA`
  (params (ActionValue :type Boolean) (ElapsedSeconds :type "Float (double-precision)") (TriggeredSeconds :type "Float (double-precision)") (InputAction :type "InputAction Object Reference" :default "/Game/Input/Controls/Jump_IA.Jump_IA"))
  (:`Triggered`
    (`self.Jump`))
  (:`Canceled`
    (`self.StopJumping`)))

(event `EnhancedInput|/Game/Input/Controls/Attack_IA`
  (params (ActionValue :type Boolean) (ElapsedSeconds :type "Float (double-precision)") (TriggeredSeconds :type "Float (double-precision)") (InputAction :type "InputAction Object Reference" :default "/Game/Input/Controls/Attack_IA.Attack_IA"))
  (:`Started`
    (`/Engine/EditorBlueprintResources/StandardMacros.DoOnce` false :!label _label
      (:`Completed`
        (`PaperZDAnimInstance.JumpToNode` (`PaperZDAnimationComponent.AnimInstance` (`self.AnimationComponent`)) "Attack" "None")
        (`KismetSystemLibrary.Delay` (`PaperFlipbookComponent.GetFlipbookLength` (`self.Sprite`)))
        (goto _label :!via `Reset`)))))

(event `EnhancedInput|/Game/Input/Controls/Pause_IA`
  (params (ActionValue :type Boolean) (ElapsedSeconds :type "Float (double-precision)") (TriggeredSeconds :type "Float (double-precision)") (InputAction :type "InputAction Object Reference" :default "/Game/Input/Controls/Pause_IA.Pause_IA"))
  (bind _returnvalue (`GameplayStatics.GetPlayerController` 0))
  (:`Started`
    (bind _returnvalue_2 (`|CreateWidget` "/Game/UI/Pausemenu_WB.Pausemenu_WB_C"))
    (`UserWidget.AddToViewport` _returnvalue_2 0)
    (set `PlayerController.bShowMouseCursor` true _returnvalue)
    (`WidgetBlueprintLibrary.SetInputMode_UIOnlyEx` _returnvalue null)
    (`GameplayStatics.SetGamePaused` true)))

(fn `Hitcheak`
  (for _array_element (`PrimitiveComponent.GetOverlappingActors` (`self.Hitbox`) "PlayerCharacter_BP_C")
    (if (!= _array_element self)
      _)))

(fn `NewFunction`
  (params (A :type "Float (double-precision)") (ScaleValue :type "Float (single-precision)"))
  (`self.AddMovementInput` (1.0 0.0 0.0) ScaleValue)
  (`Controller.SetControlRotation` (`self.GetController`) (select `bool` (> A 0.0) :`false` (`KismetMathLibrary.MakeRotator` 0.0 0.0 180.0) :`true` (`KismetMathLibrary.MakeRotator` 0.0))))

(fn `NewFunction_0`
  (bind _asplayer_controller (cast `PlayerController` (`self.GetController`)))
  (bind _returnvalue (pcsubsystem `EnhancedInputLocalPlayerSubsystem` _asplayer_controller))
  (`/Engine/EditorBlueprintResources/StandardMacros.IsValid` _returnvalue
    (:`Is Valid`
      (`EnhancedInputSubsystemInterface.AddMappingContext` _returnvalue "/Game/Input/Controls/EldenSpell_IMC.EldenSpell_IMC" 0 (struct)))))

(fn `UserConstructionScript`)