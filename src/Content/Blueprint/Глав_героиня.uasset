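; Side-scroller player character for the main heroine, with flipbook animation, horizontal movement along world X and jumping.
; Each Tick picks the jump, run or idle flipbook from falling state and velocity, then flips control rotation yaw to match X velocity.
; At zero X velocity facing falls back to Ismovingright, but the logic that sets that flag is disconnected and never runs.
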(event `self.ReceiveTick`
  (params (DeltaSeconds :type "Float (single-precision)"))
  (`self.Handle Animation`)
  (`self.Handle Rotation`))

(event `InputAction|Прыжок`
  (params (Key :type "Key Structure"))
  (:`Pressed`
    (`self.Jump`))
  (:`Released`
    (`self.StopJumping`)))

(event `InputAxis|Вправа`
  (params (AxisValue :type "Float (single-precision)"))
  (`self.AddMovementInput` (1.0 0.0 0.0) AxisValue))

(event `Handle Animation`
  (bind _sprite (`self.Sprite`))
  (if (`NavMovementComponent.IsFalling` (`self.CharacterMovement`))
    (`PaperFlipbookComponent.SetFlipbook` _sprite "/Game/Ассеты_/Персонаж/Прыжок.Прыжок")
    (else
      (`PaperFlipbookComponent.SetFlipbook` _sprite (select `bool` (> (`KismetMathLibrary.VSize` (`MovementComponent.Velocity` (`self.CharacterMovement`))) 0.0) :`false` "/Game/Ассеты_/Персонаж/Бездействие.Бездействие" :`true` "/Game/Ассеты_/Персонаж/Бег.Бег" :!type "PaperFlipbook Object Reference")))))

(event `Handle Rotation`
  (bind _velocity_x (`KismetMathLibrary.BreakVector` (`MovementComponent.Velocity` (`self.CharacterMovement`))))
  (`/Engine/EditorBlueprintResources/StandardMacros.CompareFloat` _velocity_x
    (:`>`
      (`Controller.SetControlRotation` (`self.GetController`) (`KismetMathLibrary.MakeRotator` 0.0) :!label _label))
    (:`==`
      (if (`self.ismovingright?`)
        (goto _label)
        (else
          (`Controller.SetControlRotation` (`self.GetController`) (`KismetMathLibrary.MakeRotator` 0.0 0.0 180.0) :!label _label_2))))
    (:`<`
      (goto _label_2))))

(fn `UserConstructionScript`)