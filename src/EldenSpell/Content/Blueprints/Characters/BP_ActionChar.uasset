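; BP_ActionChar is an action character with sprite animation that handles faction-based melee hits, health, stun and death.
; Its toggleable hitbox damages opposing-faction characters and briefly freezes both through CustomTimeDilation for hit stop.
; Surviving hits trigger timed stun with looping sprite shake, broadcasting stun changes.
; Lethal hits play death animation and disable capsule collision, and for players also pause into a game-over widget.
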(event `self.ReceiveBeginPlay`
  (`self.SetHitboxCollision` false)
  (set `self.CurrentHealth` (`self.MaxHealth`))
  (set `self.Sprite Base Location` (`SceneComponent.RelativeLocation` (`self.Sprite`))))

(event `self.HItbox.OnComponentBeginOverlap`
  (params (OverlappedComponent :type "PrimitiveComponent Object Reference") (OtherActor :type "Actor Object Reference") (OtherComp :type "PrimitiveComponent Object Reference") (OtherBodyIndex :type Integer) (bFromSweep :type Boolean) (SweepResult :type "HitResult Structure (by ref)"))
  (bind _asbp_action_char (cast `/Game/Blueprints/Characters/BP_ActionChar` OtherActor))
  (if (!= (`/Game/Blueprints/Characters/BP_ActionChar.Faction` _asbp_action_char) (`self.Faction`))
    (`self.ReceiveAttack` _asbp_action_char 25.0)
    (`self.Hit Stop Sequence` _asbp_action_char 0.2)
    (`self.Hit Stop Sequence` 0.2)))

(event `Hit Stop Sequence`
  (params (Duration :type "Float (single-precision)" :default 0.2))
  (set `self.CustomTimeDilation` 0.0)
  (`KismetSystemLibrary.RetriggerableDelay` Duration)
  (set `self.CustomTimeDilation` 1.0))

(event `ShakeSprite`
  (bind (_sprite_base_location_x _sprite_base_location_y _sprite_base_location_z) (`KismetMathLibrary.BreakVector` (`self.Sprite Base Location`)))
  (bind _isa (`/Engine/EditorBlueprintResources/StandardMacros.FlipFlop`)
    (:`A`
      _)
    (:`B`
      _))
  (`SceneComponent.K2_SetRelativeLocation` (`self.Sprite`) (`KismetMathLibrary.MakeVector` (+ _sprite_base_location_x (select `bool` _isa :`false` (* (`self.SpriteShakeDistance`) -1.0) :`true` (`self.SpriteShakeDistance`))) _sprite_base_location_y _sprite_base_location_z) false false))

(fn `CanAct`
  (returns (`Can Act` :type Boolean))
  (return (and (not (`self.IsAttacking`)) (not (`self.IsStunned`)) (not (`self.IsDead`)))))

(fn `ClearStun`
  (bind _output_get (set `self.IsStunned` false))
  (`self.StunStateChange` _output_get)
  (`KismetSystemLibrary.K2_ClearAndInvalidateTimerHandle` (`self.Sprite Shake Handle`))
  (`SceneComponent.K2_SetRelativeLocation` (`self.Sprite`) (`self.Sprite Base Location`) false false))

(fn `ReceiveAttack`
  (params (Damage :type "Float (double-precision)" :default 25.0))
  (if (not (`self.IsDead`))
    (set `self.CurrentHealth` (- (`self.CurrentHealth`) (`local.Damage`)))
    (`PaperZDAnimInstance.StopAllAnimationOverrides` (`self.GetAnimInstance`))
    (if (<= (`self.CurrentHealth`) 0.0)
      (if (`self.bIsPlayer`)
        (bind _returnvalue (`|CreateWidget` "/Game/Blueprints/Dead_Screen/WG_GameOver.WG_GameOver_C"))
        (`UserWidget.AddToViewport` _returnvalue 0)
        (`GameplayStatics.SetGamePaused` true)
        (set `PlayerController.bShowMouseCursor` true (`GameplayStatics.GetPlayerController` 0)))
      (`PaperZDAnimInstance.JumpToNode` (`self.GetAnimInstance`) "JumpDie" "None")
      (set `self.IsDead` true)
      (`PrimitiveComponent.SetCollisionEnabled` (`self.CapsuleComponent`) "NoCollision")
      (else
        (bind _output_get (set `self.IsStunned` true))
        (`self.StunStateChange` _output_get)
        (`PaperZDAnimInstance.StopAllAnimationOverrides` (`self.GetAnimInstance`))
        (`PaperZDAnimInstance.JumpToNode` (`self.GetAnimInstance`) "JumpStunned" "None")
        (`KismetSystemLibrary.K2_SetTimerDelegate` (`|CreateDelegate` :!event `ClearStun`) (`self.Stun Lenght`))
        (bind _returnvalue_2 (`KismetSystemLibrary.K2_SetTimerDelegate` (`|CreateDelegate` :!event `ShakeSprite`) (`self.SpriteShakeFrequncy`) true))
        (set `self.Sprite Shake Handle` _returnvalue_2)))))

(fn `SetHitboxCollision`
  (params (SetActive :type Boolean))
  (if SetActive
    (`PrimitiveComponent.SetCollisionEnabled` (`self.HItbox`) "QueryOnly")
    (else
      (`PrimitiveComponent.SetCollisionEnabled` (`self.HItbox`) "NoCollision"))))

(fn `UserConstructionScript`)